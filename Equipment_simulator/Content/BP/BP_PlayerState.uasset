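; BP_PlayerState holds the player's combat stats and rebuilds them from equipped helmet data on Status_Update.
; The update resets base values, adds helmet HP, then routes three helmet modules through ModuleCheck into flat, percentage or secondary stats.
; Percentage then derives final HP, DEF and ATK from the flat and percent totals.
; Helmet module-type counts are added last, though the reset has already zeroed them.
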(event `self.ReceiveBeginPlay`)

(event `Status_Update`
  (`self.초기화`)
  (`|ExecutionSequence`
    (:`then_0`
      ;[1 1 1] 헬멧
      (set `self.Origin_HP` (+ (`self.Origin_HP`) (`self.E_Helmet_HP`)))
      (`self.Module_Check` (`self.E_Helmet_Module_1`) (`self.E_Helmet_Module_1_Value`))
      (`self.Module_Check` (`self.E_Helmet_Module_2`) (`self.E_Helmet_Module_2_Value`))
      (`self.Module_Check` (`self.E_Helmet_Module_3`) (`self.E_Helmet_Module_3_Value`)))
    (:`then_5`
      ;[1 1 1] 퍼센트 계산
      (`|ExecutionSequence`
        (:`then_0`
          (bind _value (`self.Percentage` (`self.Origin_HP`) (`self.Percentage_HP`)))
          (set `self.HP` _value))
        (:`then_6`
          (bind _value_2 (`self.Percentage` (`self.Origin_DEF`) (`self.Percentage_DEF`)))
          (set `self.DEF` _value_2))
        (:`then_12`
          (bind _value_3 (`self.Percentage` (`self.Origin_ATK`) (`self.Percentage_ATK`)))
          (set `self.ATK` _value_3))
        (:`then_17`
          (`KismetSystemLibrary.PrintString` "업데이트 완료" true true (struct :`G` 0.66 :`B` 1.0 :`A` 1.0) 30.0))))
    (:`then_6`
      ;[1 1 1] 모듈 갯수
      (set `self.ATK_Module` (+ (`self.ATK_Module`) (`self.E_Helmet_ATK_M`)))
      (set `self.DEF_Module` (+ (`self.DEF_Module`) (`self.E_Helmet_DEF_M`)))
      (set `self.UTI_Module` (+ (`self.UTI_Module`) (`self.E_Helmet_UTI_M`))))))

(fn `Module_Check`
  (params (E_Module :type String) (E_Module_Value :type Integer))
  (switch `string` E_Module
    (:`공격력`
      (set `self.Origin_ATK` (+ (`self.Origin_ATK`) E_Module_Value)))
    (:`공격력%`
      (set `self.Percentage_ATK` (+ (`self.Percentage_ATK`) E_Module_Value)))
    (:`치명타 확률`
      (set `self.Crit` (+ (`self.Crit`) E_Module_Value)))
    (:`치명타 데미지`
      (set `self.Crit_Dmg` (+ (`self.Crit_Dmg`) E_Module_Value)))
    (:`체력`
      (set `self.Origin_HP` (+ (`self.Origin_HP`) E_Module_Value)))
    (:`체력%`
      (set `self.Percentage_HP` (+ (`self.Percentage_HP`) E_Module_Value)))
    (:`방어력`
      (set `self.Origin_DEF` (+ (`self.Origin_DEF`) E_Module_Value)))
    (:`방어력%`
      (set `self.Percentage_DEF` (+ (`self.Percentage_DEF`) E_Module_Value)))
    (:`피해감소`
      (set `self.Decrease` (+ (`self.Decrease`) E_Module_Value)))
    (:`회피율`
      (set `self.Avoid` (+ (`self.Avoid`) E_Module_Value)))
    (:`이동속도`
      (set `self.Speed` (+ (`self.Speed`) E_Module_Value)))
    (:`명중률`
      (set `self.Hitrate` (+ (`self.Hitrate`) E_Module_Value)))))

(fn `Percentage`
  (params (`Origin Value` :type Integer) (`Percentage Value` :type Integer))
  (returns (Value :type Integer))
  (return (`KismetMathLibrary.Round` (* (`KismetMathLibrary.Conv_IntToDouble` `Origin Value`) (/ (`KismetMathLibrary.Conv_IntToDouble` `Percentage Value`) 100.0)))))

(fn `UserConstructionScript`)